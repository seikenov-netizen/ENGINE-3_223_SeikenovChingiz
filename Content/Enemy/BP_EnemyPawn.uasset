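; BP_EnemyPawn is an enemy pawn that takes damage, shows a health bar and dies.
; A HealthComponent receives incoming damage and initializes the WBP_HealthBar widget at BeginPlay.
; Each tick locks the Body's world rotation and billboards the health bar toward the player camera.
; On death it prints a message, unpossesses its controller, destroys itself and spawns a fire particle at its location.
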(event `self.ReceiveBeginPlay`
  (bind _aswbp_health_bar (cast `/Game/UI/WBP_HealthBar` (`WidgetComponent.GetUserWidgetObject` (`self.HealthBarWidget`))))
  (`/Game/UI/WBP_HealthBar.InitHealthBar` _aswbp_health_bar (`self.HealthComponent`)))

(event `self.ReceiveTick`
  (params (DeltaSeconds :type "Float (single-precision)"))
  (`SceneComponent.K2_SetWorldRotation` (`self.Body`) (struct :`Pitch` -90.0) false false)
  (`SceneComponent.K2_SetWorldRotation` (`self.HealthBarWidget`) (`KismetMathLibrary.FindLookAtRotation` (`SceneComponent.K2_GetComponentLocation` (`self.HealthBarWidget`)) (`SceneComponent.K2_GetComponentLocation` (`PlayerCameraManager.TransformComponent` (`GameplayStatics.GetPlayerCameraManager` 0)))) false false))

(event `self.ReceiveAnyDamage`
  (params (Damage :type "Float (single-precision)") (DamageType :type "DamageType Object Reference") (InstigatedBy :type "Controller Object Reference") (DamageCauser :type "Actor Object Reference"))
  (`/Game/Health/HealthComponent.SetDamage` (`self.HealthComponent`) Damage))

(event `self.HealthComponent.OnDeath`
  (`KismetSystemLibrary.PrintString` "Dead" true true (struct :`G` 0.66 :`B` 1.0 :`A` 1.0) 10.0)
  (`Controller.UnPossess` (`self.GetController`))
  (`self.K2_DestroyActor`)
  (`GameplayStatics.SpawnEmitterAtLocation` "/Game/StarterContent/Particles/P_Fire.P_Fire" (`self.K2_GetActorLocation`)))

(fn `UserConstructionScript`)