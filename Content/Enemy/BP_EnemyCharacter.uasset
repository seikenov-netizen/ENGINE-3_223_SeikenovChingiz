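; BP_EnemyCharacter is an alien melee enemy that takes damage, punches the third-person player and dies with fire and sound effects.
; Damage feeds a HealthComponent, which initializes the health bar widget and drives death through OnDeath.
; StartAttackAnimation plays a swipe montage.
; ABP_Alien's punch event enables overlaps on PunchSphere, which disables them after damaging the player, limiting each opened window to a hit.
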(event `CustomEvent`
  (params (Damage :type "Float (single-precision)") (DamageType :type "DamageType Object Reference") (InstigatedBy :type "Controller Object Reference") (DamageCauser :type "Actor Object Reference"))
  (`/Game/Health/HealthComponent.SetDamage` (`self.HealthComponent`) Damage))

(event `self.HealthComponent.OnDeath`
  (`KismetSystemLibrary.PrintString` "Dead" true true (struct :`G` 0.66 :`B` 1.0 :`A` 1.0) 10.0)
  (`Controller.UnPossess` (`self.GetController`))
  (`self.K2_DestroyActor`)
  (`GameplayStatics.SpawnEmitterAtLocation` "/Game/StarterContent/Particles/P_Fire.P_Fire" (`self.K2_GetActorLocation`))
  (`GameplayStatics.PlaySoundAtLocation` "/Game/Audio/Cue/AlienDeathCue.AlienDeathCue" (`self.K2_GetActorLocation`) (struct) 1.0 1.0 0.0 null null null null))

(event `self.ReceiveBeginPlay`
  (bind _aswbp_health_bar (cast `/Game/UI/WBP_HealthBar` (`WidgetComponent.GetUserWidgetObject` (`self.HealthBarWidget`))))
  (`/Game/UI/WBP_HealthBar.InitHealthBar` _aswbp_health_bar (`self.HealthComponent`))
  (bind _asabp_alien (cast `/Game/Characters/Alien/ABP_Alien` (`SkeletalMeshComponent.GetAnimInstance` (`self.Mesh`))))
  (add `/Game/Characters/Alien/ABP_Alien.OnAttackPunch` _asabp_alien (delegate `OnAttackPunch`)))

(event `OnAttackPunch`
  (set `PrimitiveComponent.bGenerateOverlapEvents` true (`self.PunchSphere`)))

(event `self.ReceiveAnyDamage`
  (params (Damage :type "Float (single-precision)") (DamageType :type "DamageType Object Reference") (InstigatedBy :type "Controller Object Reference") (DamageCauser :type "Actor Object Reference"))
  (`/Game/Health/HealthComponent.SetDamage` (`self.HealthComponent`) Damage))

(event `self.PunchSphere.OnComponentBeginOverlap`
  (params (OverlappedComponent :type "PrimitiveComponent Object Reference") (OtherActor :type "Actor Object Reference") (OtherComp :type "PrimitiveComponent Object Reference") (OtherBodyIndex :type Integer) (bFromSweep :type Boolean) (SweepResult :type "HitResult Structure (by ref)"))
  (bind _asbp_third_person_character (cast `/Game/ThirdPerson/Blueprints/BP_ThirdPersonCharacter` OtherActor))
  (`GameplayStatics.ApplyDamage` _asbp_third_person_character 20.0 (`self.GetController`) self)
  (set `PrimitiveComponent.bGenerateOverlapEvents` false (`self.PunchSphere`)))

(event `StartAttackAnimation`
  (`|PlayMontage` (`self.Mesh`) "/Game/Characters/Alien/Animations/Mutant_Swiping_Montage.Mutant_Swiping_Montage"))

(fn `UserConstructionScript`)