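; Game mode for SurviveIO, a survival match won by staying alive for five minutes.
; On BeginPlay it starts every BP_Spawner, binds each spawned enemy's HealthComponent death to a GameState score award, and sets the victory timer inside that loop.
; The SpawnDefaultPawnAtTransform override hooks the player's death event.
; Victory unpossesses a living player; game over stops the spawners, and both print the result.
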(event `self.ReceiveBeginPlay`
  (bind _outactors (`GameplayStatics.GetAllActorsOfClass` "/Game/Enemy/BP_Spawner.BP_Spawner_C"))
  (for _array_element _outactors
    (`/Game/Enemy/BP_Spawner.OnGameStart` _array_element)
    (add `/Game/Enemy/BP_Spawner.OnEnemySpawn` _array_element (delegate `OnEnemySpawn`))
    (`KismetSystemLibrary.K2_SetTimerDelegate` (delegate `Victory`) 300.0)))

(event `OnEnemySpawn`
  (params (SpawnedActor :type "Actor Object Reference"))
  (add `/Game/Health/HealthComponent.OnDeath` (`self.GetComponentByClass` SpawnedActor "/Game/Health/HealthComponent.HealthComponent_C") (delegate `OnEnemyDeath`)))

(event `Victory`
  (if (`/Game/Health/HealthComponent.IsAlive` (`self.GetComponentByClass` (`GameplayStatics.GetPlayerPawn` 0) "/Game/Health/HealthComponent.HealthComponent_C"))
    (`Controller.UnPossess` (`GameplayStatics.GetPlayerController` 0))
    (`KismetSystemLibrary.PrintString` "VICTORY" true true (struct :`R` 0.021053 :`G` 1.0 :`A` 1.0) 20.0)
    (else
      (`self.OnGameOver`))))

(event `OnEnemyDeath`
  (bind _asgs_survive_io (cast `/Game/SurviveIO/GS_SurviveIO` (`GameplayStatics.GetGameState`)))
  (`/Game/SurviveIO/GS_SurviveIO.AddScore` _asgs_survive_io 10.0))

(event `OnPlayerDeath`
  (`self.OnGameOver`))

(event `OnGameOver`
  (`KismetSystemLibrary.PrintString` "GAME OVER" true true (struct :`R` 1.0 :`G` 0.102049 :`B` 0.098867 :`A` 1.0) 10.0)
  (bind _outactors (`GameplayStatics.GetAllActorsOfClass` "/Game/Enemy/BP_Spawner.BP_Spawner_C"))
  (for _array_element _outactors
    (`/Game/Enemy/BP_Spawner.OnGameEnd` _array_element)))

(fn `SpawnDefaultPawnAtTransform`
  (params (NewPlayer :type "Controller Object Reference") (SpawnTransform :type "Transform Structure (by ref)"))
  (returns (ReturnValue :type "Pawn Object Reference"))
  (bind _returnvalue (`parent.SpawnDefaultPawnAtTransform` NewPlayer SpawnTransform))
  (add `/Game/Health/HealthComponent.OnDeath` (`self.GetComponentByClass` _returnvalue "/Game/Health/HealthComponent.HealthComponent_C") (`|CreateDelegate` :!event `OnPlayerDeath`))
  (return _returnvalue))

(fn `UserConstructionScript`)